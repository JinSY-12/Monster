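; DefaultMonster is a monster Blueprint that chases and attacks the player character through a simple Idle, Follow, Attack state machine on Tick.
; Each tick, SaveDisAndDir caches the distance and direction to the player, which drive the range-based transitions.
; Follow moves straight toward the player via AddMovementInput, returning to Idle beyond a leash range wider than the detection range.
; Entering Attack plays the goblin slash montage once, without damage logic, and reverts to Follow when the player leaves range.
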(event Custom|SaveDisAndDir
  (bind _returnvalue (Game|GetPlayerCharacter 0))
  (bind _returnvalue_2 (Transformation|GetActorLocation))
  (bind _returnvalue_3 (Transformation|GetActorLocation _returnvalue))
  (bind _returnvalue_4 (- _returnvalue_3 _returnvalue_2))
  ;[1 1 1] 플레이어와 거리측정
  (Variables|Default|SetPlayer _returnvalue)
  (Variables|Default|SetDistancePlayerChar (Math|Vector|VectorLength _returnvalue_4))
  (Variables|Default|SetDirToPlayerChar (Math|Vector|Normalize _returnvalue_4)))

(event EventBeginPlay)

(event Collision|EventActorBeginOverlap
  (params (OtherActor :type Actor%20Object%20Reference)))

(event EventTick
  (params (DeltaSeconds :type Float%20%28single-precision%29))
  ;[1 1 1] 몬스터의 상태에 따른 행동패턴
  (CallFunction|SaveDisandDir)
  (switch Utilities|FlowControl|Switch|SwitchonMonsterStates (Variables|Default|GetCurState) ; 현재 몬스터의 상태에 따른 선택지
    (:NewEnumerator0
      (if (<= (Variables|Default|GetDistancePlayerChar) 5e+02) ; 거리 500안에 들어오면
        (Variables|Default|SetCurState "NewEnumerator1") ; 따라가는상태로 변경
      ))
    (:NewEnumerator1
      (if (<= (Variables|Default|GetDistancePlayerChar) 1.5e+02) ; 거리 80안에 들어오면
        (Variables|Default|SetCurState "NewEnumerator2") ; 공격으로 변경
        (Animation|PlayAnimMontage "/Game/Mesh/Monster/Animations/Goblin_slash_Montage.Goblin_slash_Montage" 1.0 "None")
        (else
          (Pawn|Input|AddMovementInput (Variables|Default|GetDirToPlayerChar) 1.0 false)
          (switch Utilities|FlowControl|Switch|SwitchonMonsterStates (Variables|Default|GetCurState)
            (:NewEnumerator1
              (if (> (Variables|Default|GetDistancePlayerChar) 9e+02)
                (Variables|Default|SetCurState "NewEnumerator0")))))))
    (:NewEnumerator2
      (if (> (Variables|Default|GetDistancePlayerChar) 1.5e+02)
        (Variables|Default|SetCurState "NewEnumerator1") ; 공격범위 밖으로 나가면 다시 따라가기
      ))))

(fn ConstructionScript)